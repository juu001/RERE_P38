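; Player-controlled P-38 plane pawn that flies forward constantly and drops bombs.
; Pitch and Roll axis inputs rotate the actor locally, scaled by RotationSpeed and frame delta time.
; Tick feeds forward movement input and spins the Left and Right components, likely propellers, in opposite roll directions.
; The Shoot action spawns a BP_Bomb at the Arrow component's world location.
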(event EventTick
  (params (DeltaSeconds :type Float%20%28single-precision%29))
  ;[1 1 1] right
  (Transformation|AddLocalRotation (Variables|Default|GetRight) (Math|Rotator|MakeRotator (* (Utilities|Time|GetWorldDeltaSeconds) -1e+03) 0.0 0.0) false false)
  ;[1 1 1] left
  (Transformation|AddLocalRotation (Variables|Default|GetLeft) (Math|Rotator|MakeRotator (* (Utilities|Time|GetWorldDeltaSeconds) 1e+03) 0.0 0.0) false false)
  (Pawn|Input|AddMovementInput (Transformation|GetActorForwardVector) 1.0 false))

(event Input|ActionEvents|InputActionShoot
  (params (Key :type Key%20Structure :default "None"))
  ;[1 1 1] shoot
  (:Pressed
    (Game|SpawnActorfromClass "/Game/BP/BP_Bomb.BP_Bomb_C" (Math|Transform|MakeTransform (Transformation|GetWorldLocation (Variables|Default|GetArrow)) "0, 0, 0" "1,1,1") "Undefined" 0 0)))

(event Input|AxisEvents|InputAxisPitch
  (params (AxisValue :type Float%20%28single-precision%29))
  ;[1 1 1] pitch입력
  (Transformation|AddActorLocalRotation (Math|Rotator|MakeRotator 0.0 (* AxisValue (Utilities|Time|GetWorldDeltaSeconds) (Variables|Default|GetRotationSpeed)) 0.0) false false))

(event Input|AxisEvents|InputAxisRoll
  (params (AxisValue :type Float%20%28single-precision%29))
  ;[1 1 1] roll입력
  (Transformation|AddActorLocalRotation (Math|Rotator|MakeRotator (* AxisValue (Utilities|Time|GetWorldDeltaSeconds) (Variables|Default|GetRotationSpeed)) 0.0 0.0) false false))

(fn ConstructionScript)